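; BP_Square is a flat, square level piece with a box collider, sized in the X and Y axes by its Size variable.
; The Construction Script scales ScaleRoot by Size over 100, keeping Z at 1.
; It flattens CubeMesh into a slab and sets a taller BoxCollider, raising both so their bottoms sit at zero relative height.
; The event graph has no active logic.
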(fn `UserConstructionScript`
  (bind _cube_mesh (`self.Cube Mesh`))
  (bind _box_collider (`self.Box Collider`))
  (bind (_boxextent_x _boxextent_y _boxextent_z) (`KismetMathLibrary.BreakVector` (`BoxComponent.BoxExtent` _box_collider)))
  (bind (_returnvalue_x _returnvalue_y) (`KismetMathLibrary.BreakVector` (* (1.0 1.0 0.0) (/ (`self.Size`) 100.0))))
  (`SceneComponent.SetRelativeScale3D` (`self.ScaleRoot`) (`KismetMathLibrary.MakeVector` _returnvalue_x _returnvalue_y 1.0))
  (`|ExecutionSequence`
    (:`then_0`
      (`SceneComponent.SetRelativeScale3D` _cube_mesh (1.0 1.0 0.1))
      (`SceneComponent.K2_SetRelativeLocation` (`self.Cube Mesh`) (* (`SceneComponent.RelativeScale3D` _cube_mesh) (0.0 0.0 50.0)) false false))
    (:`then_1`
      (`BoxComponent.SetBoxExtent` _box_collider (50.0 50.0 10.0) true)
      (`SceneComponent.K2_SetRelativeLocation` _box_collider (`KismetMathLibrary.MakeVector` 0.0 0.0 _boxextent_z) false false))))