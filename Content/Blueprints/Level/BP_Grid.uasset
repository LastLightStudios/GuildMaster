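; BP_Grid is a level actor that builds a tile grid and tracks which BP_Unit occupies which cell.
; Its construction script adds BP_Square child actors spaced by tile size, storing each one's grid coordinates.
; On BeginPlay, a temporary pass registers all units, deriving their cells from world position, and prints them.
; Linear searches find units or squares by coordinate; move (blocked if occupied) and swap change only stored coordinates, not transforms.
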(event `self.ReceiveBeginPlay`
  (`self.TempAssignUnits`)
  (bind _outactors (`GameplayStatics.GetAllActorsOfClass` "/Game/Blueprints/Unit/BP_Unit.BP_Unit_C"))
  (for _array_element _outactors
    (`KismetSystemLibrary.PrintString` (`KismetStringLibrary.Concat_StrStr` (`KismetSystemLibrary.GetDisplayName` _array_element) " at:" (`KismetStringLibrary.Conv_IntToString` (`/Game/Blueprints/Unit/BP_Unit.X Location` _array_element)) ", " (`KismetStringLibrary.Conv_IntToString` (`/Game/Blueprints/Unit/BP_Unit.Y Location` _array_element))))))

(fn `Build Grid`
  (locals (X :type Integer) (Y :type Integer))
  (bind (_x _y) (`KismetMathLibrary.BreakVector2D` (`self.GridSize`)))
  (bind _tile_size (defaults `/Game/Blueprints/Level/BP_Grid` (`self.SquareClass`)))
  (bind _returnvalue (/ (defaults `/Game/Blueprints/Level/BP_Grid` (`self.SquareClass`)) 2.0))
  (for _index (range (`KismetMathLibrary.FTrunc` _x))
    (set `local.X` _index)
    (for _index_2 (range (`KismetMathLibrary.FTrunc` _y))
      (set `local.Y` _index_2)
      (bind _returnvalue_2 (`AddComponent|NODE_AddChildActorComponent-0` :`RelativeTransform` (`KismetMathLibrary.MakeTransform` (`KismetMathLibrary.MakeVector` (+ (* (`local.X`) _tile_size) _returnvalue) (+ (* (`local.Y`) _tile_size) _returnvalue)))))
      (bind _asbp_square (cast `/Game/Blueprints/Level/BP_Square` (`ChildActorComponent.ChildActor` _returnvalue_2)))
      (`KismetArrayLibrary.Array_AddUnique` (`self.Squares`) _asbp_square)
      (set `/Game/Blueprints/Level/BP_Square.X Location` (`local.X`) _asbp_square)
      (set `/Game/Blueprints/Level/BP_Square.Y Location` (`local.Y`) _asbp_square))))

(fn `Find Square`
  (params (`X Location` :type Integer) (`Y Location` :type Integer))
  (returns (`Found Square` :type "/Game/Blueprints/Level/BP_Square Object Reference"))
  (locals (`Out Square` :type "/Game/Blueprints/Level/BP_Square Object Reference"))
  (set `local.Out Square` null)
  (for _array_element (`self.Squares`)
    (if (and (== `X Location` (`/Game/Blueprints/Level/BP_Square.X Location` _array_element)) (== `Y Location` (`/Game/Blueprints/Level/BP_Square.Y Location` _array_element)))
      (bind _output_get (set `local.Out Square` _array_element))
      (return _output_get))))

(fn `Find Unit`
  (params (`X Location` :type Integer) (`Y Location` :type Integer))
  (returns (`Found Unit` :type "/Game/Blueprints/Unit/BP_Unit Object Reference"))
  (locals (`Out Unit` :type "/Game/Blueprints/Unit/BP_Unit Object Reference"))
  (set `local.Out Unit` null)
  (for _array_element (`self.Units`)
    (if (and (== `X Location` (`/Game/Blueprints/Unit/BP_Unit.X Location` _array_element)) (== `Y Location` (`/Game/Blueprints/Unit/BP_Unit.Y Location` _array_element)))
      (bind _output_get (set `local.Out Unit` _array_element))
      (return _output_get))))

(fn `Move Unit`
  (params (Unit :type "/Game/Blueprints/Unit/BP_Unit Object Reference") (`Destination Square` :type "/Game/Blueprints/Level/BP_Square Object Reference"))
  (locals (`In Unit` :type "/Game/Blueprints/Unit/BP_Unit Object Reference") (`Destination X` :type Integer) (`Destination Y` :type Integer))
  (set `local.In Unit` Unit)
  (set `local.Destination X` (`/Game/Blueprints/Level/BP_Square.X Location` `Destination Square`))
  (set `local.Destination Y` (`/Game/Blueprints/Level/BP_Square.Y Location` `Destination Square`))
  (bind _found_unit (`self.Find Unit` (`local.Destination X`) (`local.Destination Y`)))
  (`/Engine/EditorBlueprintResources/StandardMacros.IsValid` _found_unit
    (:`Is Valid`
      (`KismetSystemLibrary.PrintString` "ERROR: Destination Occupied"))
    (:`Is Not Valid`
      (set `/Game/Blueprints/Unit/BP_Unit.X Location` (`local.Destination X`) (`local.In Unit`))
      (set `/Game/Blueprints/Unit/BP_Unit.Y Location` (`local.Destination Y`) (`local.In Unit`))))
  (return))

(fn `Swap Units`
  (params (`Origin Unit` :type "/Game/Blueprints/Unit/BP_Unit Object Reference") (`Destination Unit` :type "/Game/Blueprints/Unit/BP_Unit Object Reference"))
  (locals (`Origin X` :type Integer) (`Origin Y` :type Integer) (`First Unit` :type "/Game/Blueprints/Unit/BP_Unit Object Reference") (`Second Unit` :type "/Game/Blueprints/Unit/BP_Unit Object Reference"))
  (set `local.First Unit` `Origin Unit`)
  (set `local.Second Unit` `Destination Unit`)
  (`|ExecutionSequence`
    (:`then_0`
      (`KismetSystemLibrary.PrintString` "Hello")
      (set `local.Origin X` (`/Game/Blueprints/Unit/BP_Unit.X Location` (`local.First Unit`)))
      (set `local.Origin Y` (`/Game/Blueprints/Unit/BP_Unit.Y Location` (`local.First Unit`))))
    (:`then_1`
      (set `/Game/Blueprints/Unit/BP_Unit.X Location` (`/Game/Blueprints/Unit/BP_Unit.X Location` (`local.Second Unit`)) (`local.First Unit`))
      (set `/Game/Blueprints/Unit/BP_Unit.Y Location` (`/Game/Blueprints/Unit/BP_Unit.Y Location` (`local.Second Unit`)) (`local.First Unit`)))
    (:`then_2`
      (set `/Game/Blueprints/Unit/BP_Unit.X Location` (`local.Origin X`) (`local.Second Unit`))
      (set `/Game/Blueprints/Unit/BP_Unit.Y Location` (`local.Origin Y`) (`local.Second Unit`)))))

(fn `TempAssignUnits`
  (bind _tile_size (defaults `/Game/Blueprints/Level/BP_Grid` (`self.SquareClass`)))
  (bind _outactors (`GameplayStatics.GetAllActorsOfClass` "/Game/Blueprints/Unit/BP_Unit.BP_Unit_C"))
  (for _array_element _outactors
    (`KismetArrayLibrary.Array_Add` (`self.Units`) _array_element)
    (bind (_returnvalue_x _returnvalue_y) (`KismetMathLibrary.BreakVector` (/ (- (`self.K2_GetActorLocation` _array_element) (`self.K2_GetActorLocation`)) (`KismetMathLibrary.MakeVector` _tile_size _tile_size 1.0))))
    (set `/Game/Blueprints/Unit/BP_Unit.X Location` (`KismetMathLibrary.FFloor` _returnvalue_x) _array_element)
    (set `/Game/Blueprints/Unit/BP_Unit.Y Location` (`KismetMathLibrary.FFloor` _returnvalue_y) _array_element)))

(fn `UserConstructionScript`
  (`self.Build Grid`))