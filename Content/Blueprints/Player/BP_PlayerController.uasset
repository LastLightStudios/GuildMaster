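; BP_PlayerController is a player controller that handles app-level hotkeys through console commands.
; BeginPlay caches the BP_GameInstance, and input actions set a 1920x1080 resolution or exit the game.
; Two disconnected chains, which never run, would swap the Blank and NewMap streamed levels, update GamePhase, and add or remove the in-game HUD.
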(event `self.ReceiveBeginPlay`
  (bind _asbp_game_instance (cast `/Game/Blueprints/GameSystem/BP_GameInstance` (`GameplayStatics.GetGameInstance`)))
  (set `self.GameInstance` _asbp_game_instance))

(event `InputAction|SetFullScreen`
  (params (Key :type "Key Structure"))
  (:`Pressed`
    (`KismetSystemLibrary.ExecuteConsoleCommand` "r.SetRes 1920x1080" null)))

(event `InputAction|ExitGame`
  (params (Key :type "Key Structure"))
  (:`Pressed`
    (`KismetSystemLibrary.ExecuteConsoleCommand` "Exit" null)))

(event `Key|One`
  (params (Key :type "Key Structure")))

(event `Key|Two`
  (params (Key :type "Key Structure")))

(fn `UserConstructionScript`)