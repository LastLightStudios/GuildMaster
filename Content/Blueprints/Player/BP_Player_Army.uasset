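; BP_Player_Army is an actor that holds the player's army as data table row handles for units and equipped weapons.
; Its construction script calls CreateTestArmy, which appends hardcoded test entries: Rook and Pawn from DT_Units, Sword and Axe from DT_Weapons.
; The event graph has only disabled placeholder events, so the asset has no runtime logic of its own.
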(fn `CreateTestArmy`
  (`|ExecutionSequence`
    (:`then_0`
      (`KismetArrayLibrary.Array_Add` (`self.Unit Data Row Table `) (make `DataTableRowHandle` "/Game/Data/DT_Units.DT_Units" "Rook"))
      (`KismetArrayLibrary.Array_Add` (`self.Unit Data Row Table `) (make `DataTableRowHandle` "/Game/Data/DT_Units.DT_Units" "Pawn")))
    (:`then_1`
      (`KismetArrayLibrary.Array_Add` (`self.Equipped Weapons`) (make `DataTableRowHandle` "/Game/Data/DT_Weapons.DT_Weapons" "Sword"))
      (`KismetArrayLibrary.Array_Add` (`self.Equipped Weapons`) (make `DataTableRowHandle` "/Game/Data/DT_Weapons.DT_Weapons" "Axe")))))

(fn `UserConstructionScript`
  (`self.CreateTestArmy`))