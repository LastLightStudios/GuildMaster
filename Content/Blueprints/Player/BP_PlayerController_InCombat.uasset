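; Combat player controller that creates the in-game HUD and lets the player drag units between squares of a BP_Grid.
; Each tick, the cursor hit location feeds a sphere trace that updates square focus, while any held unit follows the cursor.
; Mouse release moves or swaps units through the grid and snaps their actors, returning the unit without a focused square.
; The occupancy check queries fixed square (0,0), not the focused one.
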(event `self.ReceiveBeginPlay`
  (`parent.ReceiveBeginPlay`)
  (`self.CreateInGameHUD`)
  (`self.TempFindGrid`))

(event `self.ReceiveTick`
  (params (DeltaSeconds :type "Float (single-precision)"))
  (`parent.ReceiveTick` DeltaSeconds)
  (set `self.Cursor Location` (`self.FindCursorLocation`))
  (`self.FindFocusedSquare`)
  (`self.SelectedUnitFollowsCursor`))

(event `Key|LeftMouseButton`
  (params (Key :type "Key Structure"))
  (:`Pressed`
    (`/Engine/EditorBlueprintResources/StandardMacros.IsValid` (`self.GetUnitInFocusedSquare`)
      (:`Is Valid`
        (`self.StartMovingUnit`))))
  (:`Released`
    (if (`self.Is Moving Unit`)
      (`self.StopMovingUnit`))))

(fn `CreateInGameHUD`
  (bind _returnvalue (`|CreateWidget` "/Game/Blueprints/Widget/WGT_InGameHUD.WGT_InGameHUD_C" self))
  (`UserWidget.AddToPlayerScreen` _returnvalue 0)
  (`WidgetBlueprintLibrary.SetInputMode_GameAndUIEx` self _returnvalue "DoNotLock" false)
  (set `self.bShowMouseCursor` true))

(fn `FindCursorLocation`
  (returns (`Cursor Location Hit` :type "Vector Structure"))
  (return (`.Location` (`GameplayStatics.BreakHitResult` (`self.GetHitResultUnderCursorForObjects` (`|MakeArray` "ObjectTypeQuery2" :!type "EObjectTypeQuery Enum"))))))

(fn `FindFocusedSquare`
  (bind _cursor_location (`self.Cursor Location`))
  (bind _outhits (`KismetSystemLibrary.SphereTraceMulti` _cursor_location (+ _cursor_location (0.0 0.0 1.0)) 0.0 "TraceTypeQuery3"))
  (if (> (`KismetArrayLibrary.Array_Length` _outhits) 0)
    (bind (_bblockinghit _binitialoverlap _time _distance _location _impactpoint _normal _impactnormal _physmat _hitactor) (`GameplayStatics.BreakHitResult` (`|GetArrayItem` _outhits)))
    (`/Engine/EditorBlueprintResources/StandardMacros.IsValid` _hitactor
      (:`Is Valid`
        (bind _asbp_square (cast `/Game/Blueprints/Level/BP_Square` _hitactor)
          (:`then`
            (if (!= _asbp_square (`self.Focused Square`))
              (`self.UnfocusSquare`)
              (`self.SetFocusedSquare` _asbp_square)))
          (:`CastFailed`
            (`self.UnfocusSquare` :!label _label))))
      (:`Is Not Valid`
        (goto _label)))))

(fn `GetUnitInFocusedSquare`
  (returns (`Out Unit` :type "/Game/Blueprints/Unit/BP_Unit Object Reference"))
  (locals (NewLocalVar_0 :type "/Game/Blueprints/Unit/BP_Unit Object Reference"))
  (bind _focused_square (`self.Focused Square`))
  (`/Engine/EditorBlueprintResources/StandardMacros.IsValid` _focused_square
    (:`Is Valid`
      (bind _found_unit (`/Game/Blueprints/Level/BP_Grid.Find Unit` (`self.Grid`) (`/Game/Blueprints/Level/BP_Square.X Location` _focused_square) (`/Game/Blueprints/Level/BP_Square.Y Location` _focused_square)))
      (set `local.NewLocalVar_0` _found_unit))
    (:`Is Not Valid`
      _))
  (return (`local.NewLocalVar_0`)))

(fn `SelectedUnitFollowsCursor`
  (bind (_cursor_location_x _cursor_location_y) (`KismetMathLibrary.BreakVector` (`self.Cursor Location`)))
  (bind (_returnvalue_x _returnvalue_y _returnvalue_z) (`KismetMathLibrary.BreakVector` (`self.K2_GetActorLocation` (`self.Moving Unit`))))
  (if (`self.Is Moving Unit`)
    (`self.K2_SetActorLocation` (`self.Moving Unit`) (`KismetMathLibrary.MakeVector` _cursor_location_x _cursor_location_y _returnvalue_z) false false)))

(fn `SetFocusedSquare`
  (params (`In Square` :type "/Game/Blueprints/Level/BP_Square Object Reference"))
  (bind _output_get (set `self.Focused Square` `In Square`))
  (`/Game/Blueprints/Level/BP_Square.Set Focus` _output_get 1))

(fn `StartMovingUnit`
  (set `self.Is Moving Unit` true)
  (set `self.Original Position` (`self.Focused Square`))
  (bind _output_get (set `self.Moving Unit` (`self.GetUnitInFocusedSquare`)))
  (`/Game/Blueprints/Unit/BP_Unit.SetMovingState` _output_get true)
  (`/Game/Blueprints/Unit/BP_Unit.SetFocus` _output_get true)
  (`KismetSystemLibrary.PrintString` "started moving"))

(fn `StopMovingUnit`
  (bind _moving_unit (`self.Moving Unit`))
  (`/Game/Blueprints/Unit/BP_Unit.SetMovingState` _moving_unit false)
  (`/Game/Blueprints/Unit/BP_Unit.SetFocus` _moving_unit false)
  (`/Game/Blueprints/Level/BP_Square.Set Focus` (`self.Original Position`) 0)
  (`/Engine/EditorBlueprintResources/StandardMacros.IsValid` (`self.Focused Square`)
    (:`Is Valid`
      ;[1 1 1] Is Occupied?
      (bind _found_unit (`/Game/Blueprints/Level/BP_Grid.Find Unit` (`self.Grid`) 0 0))
      (`/Engine/EditorBlueprintResources/StandardMacros.IsValid` _found_unit
        (:`Is Valid`
          ;[1 1 1] CASE: Swapping Unit with Occupied Square
          (`/Game/Blueprints/Level/BP_Grid.Swap Units` (`self.Grid`) (`self.Moving Unit`) _found_unit)
          (`self.MoveUnitLocationToSquare` (`self.Moving Unit`) (`self.Focused Square`)
            (:`Exec Out`
              (`self.MoveUnitLocationToSquare` _found_unit (`self.Original Position`)
                (:`Exec Out`
                  _)))))
        (:`Is Not Valid`
          ;[1 1 1] CASE: Move to empty Square
          (`/Game/Blueprints/Level/BP_Grid.Move Unit` (`self.Grid`) (`self.Moving Unit`) (`self.Focused Square`))
          (`self.MoveUnitLocationToSquare` (`self.Moving Unit`) (`self.Focused Square`)
            (:`Exec Out`
              _)))))
    (:`Is Not Valid`
      ;[1 1 1] CASE: Hovering Invalid Location
      (`/Game/Blueprints/Level/BP_Grid.Move Unit` (`self.Grid`) (`self.Moving Unit`) (`self.Original Position`))
      (`self.MoveUnitLocationToSquare` (`self.Moving Unit`) (`self.Original Position`)
        (:`Exec Out`
          _))))
  (set `self.Moving Unit` null)
  (set `self.Original Position` null)
  (set `self.Is Moving Unit` false))

(fn `TempFindGrid`
  (bind _outactors (`GameplayStatics.GetAllActorsOfClass` "/Game/Blueprints/Level/BP_Grid.BP_Grid_C"))
  (set `self.Grid` (`|GetArrayItem` _outactors)))

(fn `UnfocusSquare`
  (bind _original_position (`self.Original Position`))
  (`/Engine/EditorBlueprintResources/StandardMacros.IsValid` (`self.Focused Square`)
    (:`Is Valid`
      (if (== _original_position (`self.Focused Square`))
        (`/Game/Blueprints/Level/BP_Square.Set Focus` _original_position 2)
        (else
          (`/Game/Blueprints/Level/BP_Square.Set Focus` (`self.Focused Square`) 0))))))

(fn `UserConstructionScript`
  (`parent.UserConstructionScript`))