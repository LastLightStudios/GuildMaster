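; BP_Unit is a unit actor that provides visual feedback for focus and movement states.
; SetFocus toggles custom depth rendering on its static mesh and writes a fixed stencil value, which lets a post-process effect highlight it.
; SetMovingState calls a helper that shifts the mesh by a relative Z offset, raising or lowering it as moving starts or stops.
; The event graph and construction script hold no logic.
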(fn `SetFocus`
  (params (IsFocused :type Boolean))
  (if IsFocused
    (`PrimitiveComponent.SetRenderCustomDepth` (`self.StaticMesh`) true)
    (`PrimitiveComponent.SetCustomDepthStencilValue` (`self.StaticMesh`) 251)
    (else
      (`PrimitiveComponent.SetRenderCustomDepth` (`self.StaticMesh`) false))))

(fn `SetMeshRelativeZState`
  (params (`Is Being Moved` :type Boolean))
  (locals (`Z Offset` :type "Float (double-precision)" :default 100.0))
  (if `Is Being Moved`
    (`SceneComponent.K2_AddLocalOffset` (`self.StaticMesh`) (`KismetMathLibrary.MakeVector` 0.0 0.0 (`local.Z Offset`)) false false)
    (else
      (`SceneComponent.K2_AddLocalOffset` (`self.StaticMesh`) (`KismetMathLibrary.MakeVector` 0.0 0.0 (* -1 (`local.Z Offset`))) false false))))

(fn `SetMovingState`
  (params (IsBeingMoved :type Boolean))
  (`self.SetMeshRelativeZState` IsBeingMoved))

(fn `UserConstructionScript`)